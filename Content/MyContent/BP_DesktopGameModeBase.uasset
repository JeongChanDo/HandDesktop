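; Desktop game mode that shows captured screen and webcam images on in-world BP_Screen actors.
; On BeginPlay it matches each screen actor by display name to one of three screens or the webcam and gives it its own BP_MainWidget.
; Every Tick it calls ReadFrame, then pushes the screen and webcam textures into each widget's image brush.
; An older single-screen path remains but is unconnected.
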(event `self.ReceiveBeginPlay`
  (bind _outactors (`GameplayStatics.GetAllActorsOfClass` "/Game/MyContent/BP_Screen.BP_Screen_C"))
  (for _array_element _outactors
    (bind _returnvalue (`KismetSystemLibrary.GetDisplayName` _array_element))
    (if (`KismetStringLibrary.EqualEqual_StrStr` _returnvalue (`self.StrScreen1`))
      (bind _returnvalue_2 (`|CreateWidget` "/Game/MyContent/BP_MainWidget.BP_MainWidget_C"))
      (bind _output_get (set `self.Screen1` _returnvalue_2))
      (bind _screen (`/Game/MyContent/BP_Screen.Screen` _array_element))
      (`WidgetComponent.SetWidget` _screen _output_get)
      (elif (`KismetStringLibrary.EqualEqual_StrStr` _returnvalue (`self.StrScreen2`))
        (bind _returnvalue_3 (`|CreateWidget` "/Game/MyContent/BP_MainWidget.BP_MainWidget_C"))
        (bind _output_get_2 (set `self.Screen2` _returnvalue_3))
        (`WidgetComponent.SetWidget` _screen _output_get_2)
        (elif (`KismetStringLibrary.EqualEqual_StrStr` _returnvalue (`self.StrScreen3`))
          (bind _returnvalue_4 (`|CreateWidget` "/Game/MyContent/BP_MainWidget.BP_MainWidget_C"))
          (bind _output_get_3 (set `self.Screen3` _returnvalue_4))
          (`WidgetComponent.SetWidget` _screen _output_get_3)
          (elif (`KismetStringLibrary.EqualEqual_StrStr` _returnvalue (`self.StrScreenWebcam`))
            (bind _returnvalue_5 (`|CreateWidget` "/Game/MyContent/BP_MainWidget.BP_MainWidget_C"))
            (bind _output_get_4 (set `self.ScreenCam` _returnvalue_5))
            (`WidgetComponent.SetWidget` _screen _output_get_4)))))))

(event `self.ReceiveTick`
  (params (DeltaSeconds :type "Float (single-precision)"))
  (`self.ReadFrame`)
  (`Image.SetBrushFromTexture` (`/Game/MyContent/BP_MainWidget.ImageWidget` (`self.Screen1`)) (`self.imageTextureScreen1`) false)
  (`Image.SetBrushFromTexture` (`/Game/MyContent/BP_MainWidget.ImageWidget` (`self.Screen2`)) (`self.imageTextureScreen2`) false)
  (`Image.SetBrushFromTexture` (`/Game/MyContent/BP_MainWidget.ImageWidget` (`self.Screen3`)) (`self.imageTextureScreen3`) false)
  (`Image.SetBrushFromTexture` (`/Game/MyContent/BP_MainWidget.ImageWidget` (`self.ScreenCam`)) (`self.webcamTexture`) false))

(fn `UserConstructionScript`)