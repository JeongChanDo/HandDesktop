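; Right-hand actor that mirrors hand landmark data held by BP_DesktopGameModeBase, posing its HandRight mesh and moving with the hand.
; Each Tick it reads the game mode's index-keyed maps and sets every named bone's location in component space.
; The missing pinky base bone is placed midway between the wrist and landmark 17.
; The hand's X/Y values are scaled, inverted and offset onto the world YZ plane at X zero.
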(event `self.ReceiveTick`
  (params (DeltaSeconds :type "Float (single-precision)"))
  (bind _handright (`self.HandRight`))
  (bind _mapbonelocationnameright (`DesktopGameModeBase.MapBoneLocationNameRight` (stale `self.ReceiveBeginPlay` _asbp_desktop_game_mode_base)))
  (bind _keys (`BlueprintMapLibrary.Map_Keys` _mapbonelocationnameright))
  (for _array_element _keys
    (bind _value (`BlueprintMapLibrary.Map_Find` (`DesktopGameModeBase.MapBoneLocationRight` (stale `self.ReceiveBeginPlay` _asbp_desktop_game_mode_base)) _array_element))
    (`PoseableMeshComponent.SetBoneLocationByName` _handright (`KismetStringLibrary.Conv_StringToName` (`BlueprintMapLibrary.Map_Find` _mapbonelocationnameright _array_element)) _value "ComponentSpace")
    (if (== _array_element 0)
      (set `self.b_r_wrist` _value)
      (elif (== _array_element 17)
        (set `self.b_r_pinky1` _value))))
  (`PoseableMeshComponent.SetBoneLocationByName` _handright "b_r_pinky0" (/ (+ (`self.b_r_pinky1`) (`self.b_r_wrist`)) (2.0 2.0 2.0)) "ComponentSpace")
  (`self.K2_SetActorLocation` (`KismetMathLibrary.MakeVector` 0.0 (+ (* (`DesktopGameModeBase.HandRightX` (stale `self.ReceiveBeginPlay` _asbp_desktop_game_mode_base)) -2.2) 700.0) (- 600.0 (* (`DesktopGameModeBase.HandRightY` (stale `self.ReceiveBeginPlay` _asbp_desktop_game_mode_base)) 1.25)))))

(event `self.ReceiveBeginPlay`
  (bind _asbp_desktop_game_mode_base (cast `/Game/MyContent/BP_DesktopGameModeBase` (`GameplayStatics.GetGameMode`))))

(fn `UserConstructionScript`)